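; Axe weapon actor that supplies swing and area-of-effect impact feedback through callable effect events.
; On BeginPlay it caches BP_ThirdPersonGameMode, whose GameFeelControls map gates the trail, sound and impact effects so each category can be toggled.
; The swing trail is an attached Niagara system, tinted and sized at spawn and destroyed on hide.
; AOE impacts play a ground-smash sound at the axe and spawn a lightning emitter at the given location.
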(event `self.ReceiveBeginPlay`
  (`parent.ReceiveBeginPlay`)
  (bind _asbp_third_person_game_mode (cast `/Game/ThirdPerson/Blueprints/BP_ThirdPersonGameMode` (`GameplayStatics.GetGameMode`)))
  (set `self.GameModeRef` _asbp_third_person_game_mode))

(event `ShowTrailVFX`
  (if (`BlueprintMapLibrary.Map_Find` (`/Game/ThirdPerson/Blueprints/BP_ThirdPersonGameMode.GameFeelControls` (`self.GameModeRef`)) (struct :`TagName` "GameFeelControls.Weapon.TrailVFX"))
    (bind _returnvalue (`NiagaraFunctionLibrary.SpawnSystemAttached` "/Game/sA_SwordTrailSet/Fx/NS_Basic_Trail_2.NS_Basic_Trail_2" (`self.TrailVFXPoint`) "None" (0.0 0.0 0.0) (struct) "KeepRelativeOffset"))
    (bind _output_get (set `self.TrailVFXRef` _returnvalue))
    (`NiagaraComponent.SetVariableLinearColor` _output_get "Trail_Color" (make `LinearColor` 50.0 38.0 7.0 1.0))
    (`NiagaraComponent.SetVariableLinearColor` _output_get "Trail_Color_2" (make `LinearColor` 1.0 0.0 0.009094 1.0))
    (`NiagaraComponent.SetVariableLinearColor` _output_get "Trail_Color_3" (make `LinearColor` 1.0 0.890056 0.0 1.0))
    (`NiagaraComponent.SetVariableFloat` _output_get "Trail_Lifetime" 0.4)
    (`NiagaraComponent.SetVariableFloat` _output_get "Trail_Width" 75.0)))

(event `HideTrailVFX`
  (bind _trailvfxref (`self.TrailVFXRef`)
    (:`then`
      (`ActorComponent.K2_DestroyComponent` _trailvfxref))
    (:`else`)))

(event `PlaySlashSound`
  (if (`BlueprintMapLibrary.Map_Find` (`/Game/ThirdPerson/Blueprints/BP_ThirdPersonGameMode.GameFeelControls` (`self.GameModeRef`)) (struct :`TagName` "GameFeelControls.Weapon.Sound"))
    (`GameplayStatics.PlaySoundAtLocation` "/Game/Audio/Cue_AxeSwing.Cue_AxeSwing" (`self.K2_GetActorLocation`) (struct) 1.0 1.0 0.0 null null null null)))

(event `PlayAOEImpactSound`
  (if (`BlueprintMapLibrary.Map_Find` (`/Game/ThirdPerson/Blueprints/BP_ThirdPersonGameMode.GameFeelControls` (`self.GameModeRef`)) (struct :`TagName` "GameFeelControls.Impact.Sounds"))
    (`GameplayStatics.PlaySoundAtLocation` "/Game/Audio/ground-smash-explode.ground-smash-explode" (`self.K2_GetActorLocation`) (struct) 1.0 1.0 0.0 null null null null)))

(event `SpawnAOEImpactEffect`
  (params (ImpactLocation :type "Vector Structure"))
  (if (`BlueprintMapLibrary.Map_Find` (`/Game/ThirdPerson/Blueprints/BP_ThirdPersonGameMode.GameFeelControls` (`self.GameModeRef`)) (struct :`TagName` "GameFeelControls.Impact.VFX"))
    (`GameplayStatics.SpawnEmitterAtLocation` "/Game/FXVarietyPack/Particles/P_ky_lightning3.P_ky_lightning3" ImpactLocation)))

(fn `UserConstructionScript`
  (`parent.UserConstructionScript`))